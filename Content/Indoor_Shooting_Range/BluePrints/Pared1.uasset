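; Moving wall target for an indoor shooting range, worth a point when shot.
; On BeginPlay a timeline offsets it from its starting location by five times the Move value.
; A projectile hit on its collision component increments Punto1 on the first-person character and destroys the wall.
; Overlapping a ParedDestruccion actor destroys it without scoring.
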(event OnComponentHit(1puntocollision)
  (params (HitComponent :type Primitive%20Component%20Object%20Reference) (OtherActor :type Actor%20Object%20Reference) (OtherComp :type Primitive%20Component%20Object%20Reference) (NormalImpulse :type Vector :default "0, 0, 0") (Hit :type Hit%20Result%20Structure%20%28by%20ref%29))
  (Utilities|Casting|CastToFirstPersonProjectile OtherActor)
  (Utilities|FlowControl|Sequence
    (:then_0
      (bind _asfirst_person_character (Utilities|Casting|CastToFirstPersonCharacter (Game|Player|GetPlayerPawn 0)))
      (Math|Integer|IncrementInt (Variables|/Game/Indoor_Shooting_Range/Map/FirstPersonBP/Blueprints/FirstPersonCharacter.FirstPersonCharacter_C|GetPunto1 _asfirst_person_character)))
    (:then_1
      (Actor|DestroyActor))))

(event OnComponentBeginOverlap(1puntocollision)
  (params (OverlappedComponent :type Primitive%20Component%20Object%20Reference) (OtherActor :type Actor%20Object%20Reference) (OtherComp :type Primitive%20Component%20Object%20Reference) (OtherBodyIndex :type Integer) (bFromSweep :type Boolean) (SweepResult :type Hit%20Result%20Structure%20%28by%20ref%29))
  (Utilities|Casting|CastToParedDestruccion OtherActor)
  (Actor|DestroyActor))

(event EventBeginPlay
  (Variables|Default|SetPos_Inicial (Transformation|GetActorLocation))
  (bind _move (Timeline|movimientoadelante PlayFromStart)
    (:Update
      (Transformation|SetActorLocation (+ (Variables|Default|GetPos_Inicial) _move _move _move _move _move) false false))))

(event Collision|EventActorBeginOverlap
  (params (OtherActor :type Actor%20Object%20Reference)))

(event EventTick
  (params (DeltaSeconds :type Float%20%28single-precision%29)))

(fn ConstructionScript)